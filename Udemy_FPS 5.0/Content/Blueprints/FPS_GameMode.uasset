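; FPS_GameMode is the game mode that runs zombie rounds in the FPS game.
; On BeginPlay it caches FPS_GameState, gathers every EnemySpawner and starts a round, which increases the round on the game state after a short delay.
; A looping timer then has random spawners spawn zombies until the game state's zombie count reaches its spawn target, and clears itself.
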(event Custom|SpawnZombies
  (bind _gamestateref (Variables|Default|GetGameStateRef))
  (bind _enemyspawners (Variables|Default|GetEnemySpawners))
  (if (< (Variables|/Game/Blueprints/FPS_GameState.FPS_GameState_C|GetNumberOfZombies _gamestateref) (Variables|/Game/Blueprints/FPS_GameState.FPS_GameState_C|GetNumberOfZombiesToSpawn _gamestateref))
    (Default|SpawnZombie (Utilities|Array|Get(acopy) _enemyspawners (Math|Random|RandomIntegerinRange 0 (- (Utilities|Array|Length _enemyspawners) 1))))
    (else
      (Utilities|Time|ClearandInvalidateTimerbyHandle (stale Custom|StartNewRound _returnvalue)))))

(event Custom|StartNewRound
  (Utilities|FlowControl|Delay 2.0)
  (Default|IncreaseRound (Variables|Default|GetGameStateRef))
  (bind _returnvalue (Utilities|Time|SetTimerbyEvent (delegate Custom|SpawnZombies) 1.5 true)))

(event EventBeginPlay
  (bind _asfps_game_state (Utilities|Casting|CastToFPS_GameState (Game|GetGameState)))
  (Variables|Default|SetGameStateRef _asfps_game_state)
  (bind _outactors (Actor|GetAllActorsOfClass "/Game/Blueprints/Actors/EnemySpawner.EnemySpawner_C"))
  (Variables|Default|SetEnemySpawners _outactors)
  (CallFunction|StartNewRound))

(fn ConstructionScript)