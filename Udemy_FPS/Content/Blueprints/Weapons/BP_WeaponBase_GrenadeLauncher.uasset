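; Grenade launcher weapon Blueprint that extends a parent weapon class with its own ammo data and gun mesh animations.
; On BeginPlay it caches the grenade launcher ammo data from the FPS game instance.
; WeaponFire runs the parent logic, then calls the fire and reload animations on the gun mesh back to back with no delay, so reload immediately replaces fire.
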(event EventBeginPlay
  (|CallParentFunction)
  (bind _asfps_game_instance (Utilities|Casting|CastToFPS_GameInstance (Game|GetGameInstance)))
  (Variables|Default|SetAmmoData (Variables|/Game/Blueprints/FPS_GameInstance.FPS_GameInstance_C|GetGrenadeLauncherAmmoData _asfps_game_instance)))

(event EventWeaponFire
  (params (FireType :type FireType%20Enum :default "NewEnumerator0"))
  (bind _gunmesh (Variables|Default|GetGunMesh))
  (|CallParentFunction FireType)
  (Components|Animation|PlayAnimation _gunmesh "/Game/MilitaryWeapSilver/Weapons/Animations/Fire_GrenadeLauncher_W.Fire_GrenadeLauncher_W" false)
  (Components|Animation|PlayAnimation _gunmesh "/Game/MilitaryWeapSilver/Weapons/Animations/Reload_GrenadeLauncher_W.Reload_GrenadeLauncher_W" false))

(fn ConstructionScript
  (|CallParentFunction))