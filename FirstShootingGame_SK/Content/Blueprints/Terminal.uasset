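; Interactable terminal actor that fires a TerminalActivated event when the player releases Interact within ActivationDistance of its Box.
; SetPlayerInteraction gates use by storing PlayerCanInteract and enabling or disabling the actor's input for the first player controller.
; While interaction is allowed, an actor overlap shows a PlayerTip widget for a few seconds, setting the shown-once flag only after the delay ends.
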(event Collision|EventActorBeginOverlap
  (params (OtherActor :type Actor%20Object%20Reference))
  (if (and (Variables|Default|GetPlayerCanInteract) (not (Variables|Default|GetHasShownToolTip)))
    (bind _returnvalue (UserInterface|CreateWidget "/Game/UI/PlayerTip.PlayerTip_C"))
    (bind _output_get (Variables|Default|SetPlayerTip _returnvalue))
    (UserInterface|Viewport|AddtoViewport _output_get 0)
    (Utilities|FlowControl|Delay 3.0)
    (Widget|RemovefromParent _output_get)
    (Variables|Default|SetHasShownToolTip true)))

(event Input|ActionEvents|InputActionInteract
  (params (Key :type Key%20Structure :default "None"))
  (:Released
    (if (<= (Math|Vector|Distance(Vector) (Transformation|GetWorldLocation (Variables|Default|GetBox)) (Transformation|GetWorldLocation (Variables|/Script/Engine.Character|GetCapsuleComponent (Game|GetPlayerCharacter 0)))) (Variables|Default|GetActivationDistance))
      (Default|CallTerminalActivated))))

(fn ConstructionScript)

(fn SetPlayerInteraction
  (params (ShouldBeActive :type Boolean))
  (bind _returnvalue (Game|GetPlayerController 0))
  (bind _output_get (Variables|Default|SetPlayerCanInteract ShouldBeActive))
  (if _output_get
    (Input|EnableInput _returnvalue)
    (else
      (Input|DisableInput _returnvalue)))
  (return))