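; Doors is a double sliding door Blueprint that opens when its OpenDoor event is called.
; OpenDoor runs a sequence that moves RightDoor and LeftDoor apart along relative Y by MoveDistance, each after a short delay, using MoveComponentTo with rotation unchanged.
; The file contains no closing logic, and its overlap and tick events are disabled.
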(event Custom|OpenDoor
  (bind _leftdoor (Variables|Default|GetLeftDoor))
  (bind _rightdoor (Variables|Default|GetRightDoor))
  (bind _relativelocation (Variables|/Script/Engine.SceneComponent|GetRelativeLocation _rightdoor))
  (bind _relativelocation_2 (Variables|/Script/Engine.SceneComponent|GetRelativeLocation _leftdoor))
  (Utilities|FlowControl|Sequence
    (:then_0
      ;[1 1 1] Right Door Moving
      (Utilities|FlowControl|Delay 1.0)
      (Components|MoveComponentTo _rightdoor (Math|Vector|MakeVector (.x _relativelocation) (+ (.y _relativelocation) (Variables|Default|GetMoveDistance)) (.z _relativelocation)) (Variables|/Script/Engine.SceneComponent|GetRelativeRotation _rightdoor) false false 1.0 false))
    (:then_1
      ;[1 1 1] Left Door Moving
      (Utilities|FlowControl|Delay 1.0)
      (Components|MoveComponentTo _leftdoor (Math|Vector|MakeVector (.x _relativelocation_2) (- (.y _relativelocation_2) (Variables|Default|GetMoveDistance)) (.z _relativelocation_2)) (Variables|/Script/Engine.SceneComponent|GetRelativeRotation _leftdoor) false false 1.0 false))))

(event Collision|EventActorBeginOverlap
  (params (OtherActor :type Actor%20Object%20Reference)))

(event EventTick
  (params (DeltaSeconds :type Float%20%28single-precision%29)))

(fn ConstructionScript)