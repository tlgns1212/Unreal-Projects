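; RangeDummy is a target dummy, apparently for a shooting range, that reacts to weapon hits.
; ReceiveDamage ignores the incoming amount, fires OnWeaponHit and returns zero.
; OnWeaponHit calls the hit emitter, then pushes the Dummy component with an impulse from HitVelocity.
; The construction script creates a dynamic material instance on Dummy to apply its BodyColor.
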(event Custom|OnWeaponHit
  (Utilities|FlowControl|Sequence
    (:then_0
      (Default|CallOnHitEmitter))
    (:then_1
      (Physics|AddImpulse (Variables|Default|GetDummy) (Math|Conversions|ToVector(Float) (Variables|Default|GetHitVelocity)) "None" false))))

(fn ConstructionScript
  (bind _returnvalue (Rendering|Material|CreateDynamicMaterialInstance (Variables|Default|GetDummy) 0 0 "None" :!class /Script/Engine.PrimitiveComponent))
  (bind _output_get (Variables|Default|SetDynamicMaterial _returnvalue))
  (Rendering|Material|SetVectorParameterValue _output_get "BodyColor" (Variables|Default|GetBodyColor) :!class /Script/Engine.MaterialInstanceDynamic))

(fn ReceiveDamage
  (params (IncomingDamage :type Integer))
  (CallFunction|OnWeaponHit)
  (return 0))