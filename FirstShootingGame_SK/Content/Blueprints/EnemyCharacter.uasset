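; Enemy character Blueprint that gives each enemy a random dark body tint and handles its death.
; The construction script creates a dynamic material on the mesh and randomizes its BodyColor.
; After the parent damage handler runs, zero Health switches the mesh to physics, launches it by ImpulseVelocity, then destroys the actor after a delay.
; A random run-speed assignment is present but disconnected, so it never runs.
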(event EventBeginPlay)

(event EventOnReceiveDamage
  (|CallParentFunction)
  (if (<= (Variables|Default|GetHealth) 0)
    (Physics|SetSimulatePhysics (Variables|Character|GetMesh) true)
    (Physics|AddImpulse (Variables|Character|GetMesh) (Math|Conversions|ToVector(Float) (Variables|Default|GetImpulseVelocity)) "None" true)
    (Utilities|FlowControl|Delay 5.0)
    (Actor|DestroyActor)))

(fn ConstructionScript
  (bind _returnvalue (Rendering|Material|CreateDynamicMaterialInstance (Variables|Character|GetMesh) 0 0 "None" :!class /Script/Engine.PrimitiveComponent))
  (bind _output_get (Variables|Default|SetDynamicMaterial _returnvalue))
  (Rendering|Material|SetVectorParameterValue _output_get "BodyColor" (Math|Color|MakeColor (Math|Random|RandomFloatinRange 0.0 0.3) (Math|Random|RandomFloatinRange 0.0 0.3) (Math|Random|RandomFloatinRange 0.0 0.3)) :!class /Script/Engine.MaterialInstanceDynamic))