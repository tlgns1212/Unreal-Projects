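; First-person shooter character Blueprint with camera-relative movement, a hitscan gun and a reticle widget added on BeginPlay.
; Each left-click fires one camera line trace that turns a hit Ue4ASP_Character's mesh into a physics body and applies a fixed world-space impulse at the hit bone.
; Holding the button keeps the looping gun audio and muzzle flash on, gated by a DoOnce that resets on release.
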(event EventBeginPlay
  (Utilities|FlowControl|Sequence
    (:then_0
      ;[1 1 1] UI
      (bind _returnvalue (UserInterface|CreateWidget "/Game/UI/Recticle.Recticle_C" (Game|GetPlayerController 0)))
      (UserInterface|Viewport|AddtoViewport _returnvalue 0))
    (:then_1
      (Audio|Components|Audio|Stop (Variables|Default|GetGunLoop)))))

(event Input|AxisEvents|InputAxisMoveRight
  (params (AxisValue :type Float%20%28single-precision%29))
  ;[1 1 1] Movement
  (Pawn|Input|AddMovementInput (Math|Vector|GetRightVector (Variables|Default|GetCamera)) AxisValue false))

(event Input|AxisEvents|InputAxisMoveForward
  (params (AxisValue :type Float%20%28single-precision%29))
  ;[1 1 1] Movement
  (Pawn|Input|AddMovementInput (Math|Vector|GetForwardVector (Variables|Default|GetCamera)) AxisValue false))

(event Input|MouseEvents|LeftMouseButton
  (params (Key :type Key%20Structure :default "None"))
  (bind _camera (Variables|Default|GetCamera))
  (bind _returnvalue (Transformation|GetWorldLocation _camera))
  (:Pressed
    (Utilities|FlowControl|Sequence
      (:then_0
        (bind _outhit (Collision|LineTraceByChannel _returnvalue (+ _returnvalue (* (Math|Vector|GetForwardVector _camera) (Variables|Default|GetWeaponRange))) "TraceTypeQuery1" false 0 "None"))
        (bind _asue_4asp_character (Utilities|Casting|CastToUe4ASP_Character (.HitActor (Collision|BreakHitResult _outhit))))
        (Physics|SetSimulatePhysics (Variables|/Script/Engine.Character|GetMesh _asue_4asp_character) true)
        (Physics|AddImpulse (Variables|/Script/Engine.Character|GetMesh _asue_4asp_character) "1500.000000,1500.000000,0.000000" (.HitBoneName (Collision|BreakHitResult _outhit)) true))
      (:then_1
        ;[1 1 1] FX & Audio
        (Utilities|FlowControl|DoOnce false :!label _label
          (:Completed
            (Utilities|FlowControl|Sequence
              (:then_0
                (Audio|Components|Audio|Play (Variables|Default|GetGunLoop) 0.0))
              (:then_1
                (Rendering|SetVisibility (Variables|Default|GetMuzzleFlash) true false))))))))
  (:Released
    (Rendering|SetVisibility (Variables|Default|GetMuzzleFlash) false false)
    (Utilities|FlowControl|Sequence
      (:then_0
        (goto _label Reset))
      (:then_1
        (Audio|Components|Audio|Stop (Variables|Default|GetGunLoop))))))

(fn ConstructionScript)