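; Hitscan weapon Blueprint that fires a shot on FireWeapon, gated by a cooldown flag.
; Each shot plays rifle sound and muzzle flash at LaserSpawn, then clears the cooldown after the flash delay plus WeaponCooldown.
; A debug-drawn Visibility line trace along LaserSpawn's forward vector damages an EnemyCharacter hit.
; Otherwise it spawns an impact effect, followed by a delayed sound call with no sound asset set.
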(event Custom|FireWeapon
  (bind _laserspawn (Variables|Default|GetLaserSpawn))
  (bind _laserspawn_2 (Variables|Default|GetLaserSpawn))
  (bind _returnvalue (Transformation|GetWorldLocation _laserspawn))
  ;[1 1 1] Fire Weapon
  (if (not (Variables|Default|GetCooldown))
    (Utilities|FlowControl|Sequence
      (:then_0
        ;[1 1 1] Sound & FX
        (Utilities|FlowControl|Sequence
          (:then_0
            (Audio|SpawnSoundAttached "/Game/Audio/AssaultRifle_Shot06_Stereo.AssaultRifle_Shot06_Stereo" _laserspawn_2 "None" "0, 0, 0" "0, 0, 0" "KeepRelativeOffset" false 1.0 1.0 0.0 0 0))
          (:then_1
            (bind _returnvalue_2 (Effects|SpawnEmitterAttached "/Game/GunFX/ParticleSystems/Weapons/AssaultRifle/Muzzle/P_AssaultRifle_MF.P_AssaultRifle_MF" _laserspawn_2 "None" (Transformation|GetWorldLocation _laserspawn_2) (Transformation|GetWorldRotation _laserspawn_2) "1.000000,1.000000,1.000000" "KeepWorldPosition"))
            (Utilities|FlowControl|Delay 0.2)
            (Components|DestroyComponent _returnvalue_2)
            (Utilities|FlowControl|Delay (Variables|Default|GetWeaponCooldown))
            (Variables|Default|SetCooldown false))))
      (:then_1
        (Variables|Default|SetCooldown true))
      (:then_2
        ;[1 1 1] Bullets (Raycasting)
        (bind _outhit (Collision|LineTraceByChannel _returnvalue (+ _returnvalue (* (Math|Vector|GetForwardVector (Transformation|GetWorldRotation _laserspawn)) (Math|Conversions|ToVector(Float) (Variables|Default|GetWeaponRange)))) "TraceTypeQuery1" false 0 "ForOneFrame"))
        (bind _output_get (Variables|Default|SetHitActor (.HitActor (Collision|BreakHitResult _outhit))))
        (bind _asenemy_character (Utilities|Casting|CastToEnemyCharacter _output_get)
          (:then
            (Default|ReceiveDamage _asenemy_character (Variables|Default|GetWeaponDamage)))
          (:CastFailed
            (Effects|SpawnEmitteratLocation "/Game/GunFX/ParticleSystems/Weapons/AssaultRifle/Impacts/P_AssaultRifle_IH.P_AssaultRifle_IH" (.ImpactPoint (Collision|BreakHitResult _outhit)) (Math|Conversions|RotationFromXVector (.ImpactNormal (Collision|BreakHitResult _outhit))))
            (Utilities|FlowControl|Delay 0.5)
            (Audio|SpawnSoundatLocation 0 (.ImpactPoint (Collision|BreakHitResult _outhit)) "0, 0, 0" 1.0 1.0 0.0 0 0)))))))

(fn ConstructionScript)