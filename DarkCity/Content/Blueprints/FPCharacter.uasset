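; First-person player character that carries a spawned flashlight and recharges it by overlapping battery pickups, which are then destroyed.
; On begin play it attaches the flashlight to a socket using a placeholder mesh's transform, hides the placeholder and creates the HUD.
; Movement follows camera axes, while look comes from axis inputs or touch drags on the right half of the screen.
; Vertical look and touch drags update the flashlight socket's pitch from control rotation.
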(event Custom|RotateFlashlight
  (bind _flashsocket (Variables|Default|GetFlashSocket))
  (bind _relativelocation (Variables|/Script/Engine.SceneComponent|GetRelativeLocation _flashsocket))
  ;[1 1 1] Flashlight Rotation
  (Transformation|SetRelativeRotation _flashsocket (Math|Rotator|MakeRotator (.x _relativelocation) (.pitch (Pawn|GetControlRotation :!class /Script/Engine.Pawn)) (.z _relativelocation)) false false))

(event Custom|SpawnFlashlight
  (bind _flashlightstatic (Variables|Default|GetFlashLightStatic))
  (bind _returnvalue (Transformation|GetRelativeTransform _flashlightstatic))
  ;[1 1 1] Spawn Flashlight
  (bind _returnvalue_2 (Game|SpawnActorfromClass "/Game/Blueprints/Flashlight.Flashlight_C" (Transformation|GetActorTransform) "AlwaysSpawn" 0 0))
  (bind _output_get (Variables|Default|SetFlashLight _returnvalue_2))
  (Transformation|AttachComponentToComponent (Variables|/Script/Engine.Actor|GetRootComponent _output_get) (Variables|Default|GetFlashSocket) "None" "KeepRelative" "KeepRelative" "KeepRelative" true)
  (Transformation|SetActorRelativeTransform (Variables|Default|GetFlashLight) (Math|Transform|MakeTransform (.location _returnvalue) (.rotation _returnvalue)) false false)
  (Rendering|SetVisibility _flashlightstatic false false))

(event Custom|CreateUI
  ;[1 1 1] Create UI
  (bind _returnvalue (UserInterface|CreateWidget "/Game/UI/PlayerHUD.PlayerHUD_C" (Game|GetPlayerController 0)))
  (bind _output_get (Variables|Default|SetHUD _returnvalue))
  (UserInterface|Viewport|AddtoViewport _output_get 0))

(event EventBeginPlay
  ;[1 1 1] Begin Play
  (Utilities|FlowControl|Sequence
    (:then_0
      (CallFunction|SpawnFlashlight))
    (:then_1
      (CallFunction|CreateUI))))

(event Collision|EventActorBeginOverlap
  (params (OtherActor :type Actor%20Object%20Reference))
  ;[1 1 1] Battery Pickup
  (bind _asbatteries (Utilities|Casting|CastToBatteries OtherActor))
  (Default|ChargeBattery (Variables|Default|GetFlashLight))
  (Actor|DestroyActor _asbatteries))

(event Input|AxisEvents|InputAxisMoveForward
  (params (AxisValue :type Float%20%28single-precision%29))
  ;[1 1 1] Input Movement
  (Pawn|Input|AddMovementInput (Math|Vector|GetForwardVector (Variables|Default|GetCamera)) AxisValue false))

(event Input|AxisEvents|InputAxisMoveRight
  (params (AxisValue :type Float%20%28single-precision%29))
  ;[1 1 1] Input Movement
  (Pawn|Input|AddMovementInput (Math|Vector|GetRightVector (Variables|Default|GetCamera)) AxisValue false))

(event Input|AxisEvents|InputAxisLookRight
  (params (AxisValue :type Float%20%28single-precision%29))
  ;[1 1 1] Input Editor Look
  (Pawn|Input|AddControllerYawInput AxisValue))

(event Input|AxisEvents|InputAxisLookUp
  (params (AxisValue :type Float%20%28single-precision%29))
  ;[1 1 1] Input Editor Look
  (Pawn|Input|AddControllerPitchInput AxisValue)
  (CallFunction|RotateFlashlight))

(event Input|TouchEvents|InputTouch
  (params (Location :type Vector) (FingerIndex :type ETouchIndex%20Enum))
  ;[1 1 1] Input Touch Look
  (:Pressed
    (bind _isvalid (CallFunction|IsLookTouchLocationValid Location :!label _label))
    (if _isvalid
      (Variables|Default|SetLastTouchLocation Location)))
  (:Released
    (goto _label))
  (:Moved
    (bind _isvalid_2 (CallFunction|IsLookTouchLocationValid Location))
    (if (and _isvalid_2 (or (Utilities|Enum|Equal(Enum) FingerIndex "Touch1") (Utilities|Enum|Equal(Enum) FingerIndex "Touch2")))
      (Pawn|Input|AddControllerYawInput (* (Variables|Default|GetLookSpeedMinus) (.X (Math|Vector|BreakVector (- (Variables|Default|GetLastTouchLocation) Location)))))
      (Pawn|Input|AddControllerPitchInput (* (Variables|Default|GetLookSpeedMinus) (.Y (Math|Vector|BreakVector (- (Variables|Default|GetLastTouchLocation) Location)))))
      (Variables|Default|SetLastTouchLocation Location)
      (CallFunction|RotateFlashlight))))

(fn ConstructionScript)

(fn IsLookTouchLocationValid
  (params (LastTouchLocation :type Vector))
  (return (> (.X (Math|Vector|BreakVector LastTouchLocation)) (/ (.x (Viewport|GetViewportSize)) 2.0))))