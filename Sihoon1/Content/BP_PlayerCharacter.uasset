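; Player character Blueprint that turns player input into movement, look, jump, sprint and crouch actions.
; Forward and right axes add movement along directions derived from control rotation yaw only, so pitch does not affect walking.
; Look axes feed controller pitch and yaw.
; Jump and crouch act while their keys are held, and sprint swaps the movement component's max walk speed between sprint and normal values.
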(event Input|ActionEvents|InputActionJumpKey
  (params (Key :type Key%20Structure :default "None"))
  ;[1 1 1] JumpAction
  (:Pressed
    (Character|Jump))
  (:Released
    (Character|StopJumping)))

(event Input|ActionEvents|InputActionSprintKey
  (params (Key :type Key%20Structure :default "None"))
  (bind _charactermovement (Variables|Character|GetCharacterMovement))
  ;[1 1 1] SprintAction
  (:Pressed
    (Variables|/Script/Engine.CharacterMovementComponent|SetMaxWalkSpeed _charactermovement (Variables|Default|GetSprintWalkSpeed)))
  (:Released
    (Variables|/Script/Engine.CharacterMovementComponent|SetMaxWalkSpeed _charactermovement (Variables|Default|GetNormalWalkSpeed))))

(event Input|ActionEvents|InputActionCrouchKey
  (params (Key :type Key%20Structure :default "None"))
  ;[1 1 1] CrouchAction
  (:Pressed
    (Character|Crouch))
  (:Released
    (Character|UnCrouch)))

(event Input|AxisEvents|InputAxisMoveForwardKey
  (params (AxisValue :type Float%20%28single-precision%29))
  ;[1 1 1] MovementInput
  (Pawn|Input|AddMovementInput (Math|Vector|GetForwardVector (Math|Rotator|MakeRotator 0.0 0.0 (.yaw (Pawn|GetControlRotation :!class /Script/Engine.Pawn)))) AxisValue false))

(event Input|AxisEvents|InputAxisMoveRightKey
  (params (AxisValue :type Float%20%28single-precision%29))
  ;[1 1 1] MovementInput
  (Pawn|Input|AddMovementInput (Math|Vector|GetRightVector (Math|Rotator|MakeRotator 0.0 0.0 (.yaw (Pawn|GetControlRotation :!class /Script/Engine.Pawn)))) AxisValue false))

(event Input|AxisEvents|InputAxisLookUpKey
  (params (AxisValue :type Float%20%28single-precision%29))
  ;[1 1 1] MouseInput
  (Pawn|Input|AddControllerPitchInput AxisValue))

(event Input|AxisEvents|InputAxisTurnKey
  (params (AxisValue :type Float%20%28single-precision%29))
  ;[1 1 1] MouseInput
  (Pawn|Input|AddControllerYawInput AxisValue))

(fn ConstructionScript)