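; Player character Blueprint handling movement, look, sprint, crouch, jump and weapon use.
; Keys 1 and 2 spawn a rifle or pistol onto a mesh socket, only while unarmed.
; Fire delegates to the current weapon and broadcasts to listeners, auto-reloading empty magazines when spare ammo remains.
; Equip and reload timelines drive WeaponPullDownAlpha, with state flags gating firing and letting equipping cancel reloads.
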(event Custom|EquipWeapon
  (params (Weapon :type BP%20Weapon%20Base%20Object%20Reference))
  ;[1 1 1] EquipWeapon Event
  (if (not (Variables|Weapon|GetIsChangingWeapon))
    (if (Variables|Weapon|GetIsReloading)
      (Variables|Weapon|SetIsCanFire false)
      (Variables|Weapon|SetIsReloading false))
    (Variables|Weapon|SetIsChangingWeapon true)
    (bind _animpercentage (Timeline|EquipWeaponTimeline Play)
      (:Update
        (Variables|Default|SetWeaponPullDownAlpha _animpercentage))
      (:Finished
        (Variables|Weapon|SetIsChangingWeapon false)
        (Variables|Weapon|SetIsCanFire true))
      (:WeaponSwitch
        (CallFunction|ShowWeapons Weapon)
        (Variables|Weapon|SetCurrentWeapon Weapon)
        (Variables|Weapon|SetHasWeaponEnum "NewEnumerator1")))))

(event Custom|StopFire
  ;[1 1 1] StopFire Event
  (Default|CallCharacterStopFireWeapon))

(event Custom|Reload
  ;[1 1 1] Reload Event
  (if (not (Variables|Weapon|GetIsReloading))
    (Variables|Weapon|SetIsReloading true)
    (Variables|Weapon|SetIsCanFire false)
    (bind _alpha (Timeline|ReloadingPullDown PlayFromStart)
      (:Update
        (if (Variables|Weapon|GetIsReloading)
          (Variables|Default|SetWeaponPullDownAlpha _alpha)))
      (:Finished
        (if (Variables|Weapon|GetIsReloading)
          (Utilities|FlowControl|Delay (Variables|/Game/BluePrints/Weapons/BP_WeaponBase.BP_WeaponBase_C|GetReloadTime (Variables|Weapon|GetCurrentWeapon)))
          (bind _alpha_2 (Timeline|WeaponPullUp PlayFromStart)
            (:Update
              (if (Variables|Weapon|GetIsReloading)
                (Variables|Default|SetWeaponPullDownAlpha _alpha_2)))
            (:Finished
              (if (Variables|Weapon|GetIsReloading)
                (Default|WeaponReload (Variables|Weapon|GetCurrentWeapon))
                (Variables|Weapon|SetIsReloading false)
                (Variables|Weapon|SetIsCanFire true)))))))))

(event Custom|Fire
  (bind _currentweapon (Variables|Weapon|GetCurrentWeapon))
  (bind _currentweapon_2 (Variables|Weapon|GetCurrentWeapon))
  ;[1 1 1] Fire Event
  (if (Variables|Weapon|GetIsCanFire)
    (if (.IsHasAmmo (Default|HasAmmoinMag _currentweapon_2))
      (Default|WeaponFire _currentweapon)
      (Default|CallCharacterFireWeapon (Variables|/Game/BluePrints/Weapons/BP_WeaponBase.BP_WeaponBase_C|GetWeaponType _currentweapon))
      (elif (Default|HasExtraAmmo _currentweapon_2)
        (CallFunction|Reload)
        (else
          (Development|PrintString "no ammo"))))))

(event Input|ActionEvents|InputActionJumpKey
  (params (Key :type Key%20Structure :default "None"))
  ;[1 1 1] JumpAction
  (:Pressed
    (if (Variables|Movement|GetisCrouch)
      (Character|UnCrouch)
      (Utilities|FlowControl|Delay 0.001)
      (Character|Jump)
      (Utilities|FlowControl|Delay 0.9)
      (if (Variables|Movement|GetisCrouch)
        (Character|Crouch))
      (else
        (Character|Jump))))
  (:Released
    (Character|StopJumping)))

(event Input|ActionEvents|InputActionSprintKey
  (params (Key :type Key%20Structure :default "None"))
  (bind _charactermovement (Variables|Character|GetCharacterMovement))
  ;[1 1 1] SprintAction
  (:Pressed
    (Variables|/Script/Engine.CharacterMovementComponent|SetMaxWalkSpeed _charactermovement (Variables|Movement|GetSprintWalkSpeed)))
  (:Released
    (Variables|/Script/Engine.CharacterMovementComponent|SetMaxWalkSpeed _charactermovement (Variables|Movement|GetNormalWalkSpeed))))

(event Input|ActionEvents|InputActionCrouchKey
  (params (Key :type Key%20Structure :default "None"))
  ;[1 1 1] CrouchAction
  (:Pressed
    (Variables|Movement|SetisCrouch true)
    (Character|Crouch))
  (:Released
    (Variables|Movement|SetisCrouch false)
    (Character|UnCrouch)))

(event Input|ActionEvents|InputActionFire
  (params (Key :type Key%20Structure :default "None"))
  (bind _hasweaponenum (Variables|Weapon|GetHasWeaponEnum))
  ;[1 1 1] InputKeyboadActions
  (:Pressed
    (switch Utilities|FlowControl|Switch|SwitchonHasWeapon _hasweaponenum
      (:NewEnumerator0
        (Development|PrintString "No Weapon" :!label _label))
      (:NewEnumerator1
        (CallFunction|Fire))))
  (:Released
    (switch Utilities|FlowControl|Switch|SwitchonHasWeapon _hasweaponenum
      (:NewEnumerator0
        (goto _label))
      (:NewEnumerator1
        (CallFunction|StopFire)))))

(event Input|ActionEvents|InputActionReload
  (params (Key :type Key%20Structure :default "None"))
  ;[1 1 1] InputKeyboadActions
  (:Pressed
    (switch Utilities|FlowControl|Switch|SwitchonHasWeapon (Variables|Weapon|GetHasWeaponEnum)
      (:NewEnumerator0
        (Development|PrintString "No Weapon"))
      (:NewEnumerator1
        (if (not (or (Variables|Weapon|GetIsReloading) (Variables|Weapon|GetIsChangingWeapon)))
          (if (not (.IsMagFull (Default|HasAmmoinMag (Variables|Weapon|GetCurrentWeapon))))
            (CallFunction|Reload)))))))

(event Input|AxisEvents|InputAxisMoveForwardKey
  (params (AxisValue :type Float%20%28single-precision%29))
  ;[1 1 1] MovementInput
  (Pawn|Input|AddMovementInput (Math|Vector|GetForwardVector (Math|Rotator|MakeRotator 0.0 0.0 (.yaw (Pawn|GetControlRotation :!class /Script/Engine.Pawn)))) AxisValue false))

(event Input|AxisEvents|InputAxisMoveRightKey
  (params (AxisValue :type Float%20%28single-precision%29))
  ;[1 1 1] MovementInput
  (Pawn|Input|AddMovementInput (Math|Vector|GetRightVector (Math|Rotator|MakeRotator 0.0 0.0 (.yaw (Pawn|GetControlRotation :!class /Script/Engine.Pawn)))) AxisValue false))

(event Input|AxisEvents|InputAxisLookUpKey
  (params (AxisValue :type Float%20%28single-precision%29))
  ;[1 1 1] MouseInput
  (Pawn|Input|AddControllerPitchInput AxisValue))

(event Input|AxisEvents|InputAxisTurnKey
  (params (AxisValue :type Float%20%28single-precision%29))
  ;[1 1 1] MouseInput
  (Pawn|Input|AddControllerYawInput AxisValue))

(event Input|KeyboardEvents|1
  (params (Key :type Key%20Structure :default "None"))
  ;[1 1 1] InputKeyboadActions
  (:Pressed
    (if (Utilities|Enum|Equal(Enum) (Variables|Weapon|GetHasWeaponEnum) "NewEnumerator0")
      (bind _weaponref (CallFunction|SpawnWeapons "/Game/BluePrints/Weapons/BP_WeaponBase_AssaultRifle.BP_WeaponBase_AssaultRifle_C"))
      (CallFunction|EquipWeapon _weaponref))))

(event Input|KeyboardEvents|2
  (params (Key :type Key%20Structure :default "None"))
  ;[1 1 1] InputKeyboadActions
  (:Pressed
    (if (Utilities|Enum|Equal(Enum) (Variables|Weapon|GetHasWeaponEnum) "NewEnumerator0")
      (bind _weaponref (CallFunction|SpawnWeapons "/Game/BluePrints/Weapons/BP_WeaponBase_Pistol.BP_WeaponBase_Pistol_C"))
      (CallFunction|EquipWeapon _weaponref))))

(fn ConstructionScript)

(fn ShowWeapons
  (params (Weapon :type BP%20Weapon%20Base%20Object%20Reference))
  (bind _output_get (LocalVariables|SetLocalWeaponToShow Weapon))
  (bind _output_get_2 (Variables|Weapon|SetWeaponSlot_01 _output_get))
  (Rendering|SetActorHiddenInGame _output_get_2 false))

(fn SpawnWeapons
  (params (Weapon :type BP%20Weapon%20Base%20Class%20Reference))
  (bind _output_get (Variables|Default|SetLocalWeaponClassToSpawn Weapon))
  (bind _returnvalue (Game|SpawnActorfromClass _output_get (Transformation|GetActorTransform) "Undefined" 0 0))
  (bind _output_get_2 (Variables|Weapon|SetWeaponSlot_01 _returnvalue))
  (Transformation|AttachComponentToComponent _output_get_2 (Variables|Character|GetMesh) (Variables|/Game/BluePrints/Weapons/BP_WeaponBase.BP_WeaponBase_C|GetSocketName _returnvalue) "SnapToTarget" "SnapToTarget" "SnapToTarget" false)
  (Variables|Weapon|SetCurrentWeapon (Variables|Weapon|GetWeaponSlot_01))
  (Variables|Weapon|SetHasWeaponEnum "NewEnumerator1")
  (return _returnvalue))