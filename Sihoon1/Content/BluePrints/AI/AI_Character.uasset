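; AI character Blueprint that takes hit and radius damage, tracks health and dies.
; Direct hits apply a random critical roll and a physical-material multiplier via DestructibleDamageThresholdScale, while radius damage scales linearly with distance from the impact.
; Both paths update health, then spawn jittered screen-projected damage numbers and a hitmarker.
; Death sets the blackboard isDead flag, ragdolls the mesh with a weapon-based impulse away from the player, and removes the capsule.
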(event EventTakeRadiusDamage
  (params (GroundHitResult :type Hit%20Result%20Structure) (AmmoData :type Ammo%20Data%20Structure) (CriticalHitDamageModifier :type Float%20%28double-precision%29))
  (bind (_damage _criticalhitchance _speed _damageradius) (Utilities|Struct|BreakAmmoData AmmoData))
  (bind (_bblockinghit _binitialoverlap _time _distance _location _impactpoint _normal _impactnormal _physmat _hitactor _hitcomponent _hitbonename) (Collision|BreakHitResult GroundHitResult))
  ;[1 1 1] Take Radius Damage
  (if (not (Variables|Default|GetIsDead))
    (bind _damagetoapply (CallFunction|SetRadiusDamage :Damage _damage :CriticalDamageModifier 1.0 :Radius _damageradius :GroundPoint _impactpoint))
    (bind _isdead (CallFunction|UpdateHealth _damagetoapply))
    (bind _output_get (Variables|Default|SetIsDead _isdead))
    (if _output_get
      (CallFunction|Die _impactpoint _hitbonename))
    (CallFunction|FloatingDamage _damagetoapply _impactpoint)
    ;[1 1 1] Hitmarks
    (Utilities|IsValid (Variables|Default|GetHitmarkerRef)
      (:Is%20Valid
        (Widget|RemovefromParent (Variables|Default|GetHitmarkerRef)))
      (:Is%20Not%20Valid
        _))
    (bind _returnvalue (UserInterface|CreateWidget "/Game/BluePrints/UMG/UI_Hitmarker.UI_Hitmarker_C" 0 (Variables|Default|GetIsDead)))
    (bind _output_get_2 (Variables|Default|SetHitmarkerRef _returnvalue))
    (UserInterface|Viewport|AddtoViewport _output_get_2 0)))

(event EventFloatingDamage
  (params (Damage :type Float%20%28double-precision%29) (ImpactPoint :type Vector :default "0, 0, 0"))
  (bind _returnvalue (Game|GetPlayerController 0))
  (bind _screenposition (Class|WidgetLayoutLibrary|ProjectWorldLocationtoWidgetPosition _returnvalue ImpactPoint false))
  (bind (_x _y) (Math|Vector2D|BreakVector2D _screenposition))
  ;[1 1 1] Floating Damage
  (bind _returnvalue_2 (UserInterface|CreateWidget "/Game/BluePrints/UMG/UI_FloatingDamage.UI_FloatingDamage_C" 0 Damage))
  (Class|Widget|SetRenderTranslation (Variables|/Game/BluePrints/UMG/UI_FloatingDamage.UI_FloatingDamage_C|GetScreenPositionSizeBox _returnvalue_2) (Math|Vector2D|MakeVector2D (+ (+ _x -5e+01) (Math|Random|RandomFloatinRange -25.0 25.0)) (+ (+ _y -1e+02) (Math|Random|RandomFloatinRange -1e+01 1e+01))))
  (UserInterface|Viewport|AddtoViewport _returnvalue_2 0))

(event EventBeginPlay
  (bind _asbp_player_character (Utilities|Casting|CastToBP_PlayerCharacter (Game|Player|GetPlayerPawn 0)))
  (Variables|Default|SetPlayerRef _asbp_player_character))

(event EventTakeDamage
  (params (AmmoData :type Ammo%20Data%20Structure) (CriticalDamageModifier :type Float%20%28double-precision%29) (HitResult :type Hit%20Result%20Structure))
  (bind (_damage _criticalhitchance) (Utilities|Struct|BreakAmmoData AmmoData))
  (bind (_bblockinghit _binitialoverlap _time _distance _location _impactpoint _normal _impactnormal _physmat _hitactor _hitcomponent _hitbonename) (Collision|BreakHitResult HitResult))
  ;[1 1 1] Take Damage
  (bind _damagetoapply (CallFunction|SetDamage _damage _criticalhitchance CriticalDamageModifier HitResult))
  (Development|PrintString (Utilities|String|ToString(Float) _damagetoapply))
  (bind _isdead (CallFunction|UpdateHealth _damagetoapply))
  (bind _output_get (Variables|Default|SetIsDead _isdead))
  (if _output_get
    (CallFunction|Die _impactpoint _hitbonename))
  (CallFunction|FloatingDamage _damagetoapply _impactpoint)
  ;[1 1 1] Hitmarks
  (Utilities|IsValid (Variables|Default|GetHitmarkerRef)
    (:Is%20Valid
      (Widget|RemovefromParent (Variables|Default|GetHitmarkerRef)))
    (:Is%20Not%20Valid
      _))
  (bind _returnvalue (UserInterface|CreateWidget "/Game/BluePrints/UMG/UI_Hitmarker.UI_Hitmarker_C" 0 (Variables|Default|GetIsDead)))
  (bind _output_get_2 (Variables|Default|SetHitmarkerRef _returnvalue))
  (UserInterface|Viewport|AddtoViewport _output_get_2 0))

(fn ConstructionScript)

(fn SetDamage
  (params (Damage :type Float%20%28double-precision%29) (CriticalHitChance :type Float%20%28double-precision%29) (CriticalDamageModifier :type Float%20%28double-precision%29) (HitResult :type Hit%20Result%20Structure))
  (LocalVariables|SetLocalDamageAmt Damage)
  (Utilities|FlowControl|Sequence
    (:then_0
      (bind _output_get (LocalVariables|SetLocalIsCriticalHit (< CriticalHitChance (Math|Random|RandomFloatinRange 0.0 1e+02))))
      (if _output_get
        (LocalVariables|SetLocalDamageAmt (* (LocalVariables|GetLocalDamageAmt) CriticalDamageModifier))))
    (:then_1
      (LocalVariables|SetLocalDamageAmt (* (Variables|/Script/PhysicsCore.PhysicalMaterial|GetDestructibleDamageThresholdScale (.PhysMat (Collision|BreakHitResult HitResult))) (LocalVariables|GetLocalDamageAmt))))
    (:then_2
      (return (LocalVariables|GetLocalDamageAmt) (LocalVariables|GetLocalIsCriticalHit)))))

(fn UpdateHealth
  (params (Damage :type Float%20%28double-precision%29))
  (Utilities|FlowControl|Sequence
    (:then_0
      (if (>= Damage (Variables|Default|GetCurrentHealth))
        (LocalVariables|SetLocalIsDead true)
        (Variables|Default|SetCurrentHealth 0.0)
        (else
          (Variables|Default|SetCurrentHealth (- (Variables|Default|GetCurrentHealth) Damage)))))
    (:then_1
      (return (LocalVariables|GetLocalIsDead)))))

(fn SetRadiusDamage
  (params (Damage :type Float%20%28double-precision%29) (CriticalHitChance :type Float%20%28double-precision%29) (CriticalDamageModifier :type Float%20%28double-precision%29) (HitResult :type Hit%20Result%20Structure) (Radius :type Float%20%28double-precision%29) (GroundPoint :type Vector))
  (LocalVariables|SetLocalDamageAmt Damage)
  (Utilities|FlowControl|Sequence
    (:then_0
      (bind _output_get (LocalVariables|SetLocalIsCriticalHit (< CriticalHitChance (Math|Random|RandomFloatinRange 0.0 1e+02))))
      (if _output_get
        (LocalVariables|SetLocalDamageAmt (* (LocalVariables|GetLocalDamageAmt) CriticalDamageModifier))))
    (:then_1
      (return (* (- 1.0 (/ (Math|Vector|VectorLength (- GroundPoint (Transformation|GetActorLocation))) Radius)) (LocalVariables|GetLocalDamageAmt)) (LocalVariables|GetLocalIsCriticalHit)))))

(fn Die
  (params (ImpactPoint :type Vector) (BoneName :type Name))
  (bind _mesh (Variables|Character|GetMesh))
  (bind _playerref (Variables|Default|GetPlayerRef))
  (bind _capsulecomponent (Variables|Collision|GetCapsuleComponent))
  (AI|Components|Blackboard|SetValueasBool (AI|GetBlackboard (Pawn|GetController)) (Utilities|Name|MakeLiteralName "isDead") true)
  (Physics|SetSimulatePhysics _mesh true)
  (Physics|AddImpulseatLocation _mesh (* (Math|Vector|GetUnitDirection(Vector) (Transformation|GetActorLocation _playerref) (Transformation|GetActorLocation)) (Utilities|Select :Index (Variables|/Game/BluePrints/Characters/BP_PlayerCharacter.BP_PlayerCharacter_C|GetHasWeaponEnum _playerref) :NewEnumerator0 1e+04 :NewEnumerator1 (Variables|/Game/BluePrints/Weapons/BP_WeaponBase.BP_WeaponBase_C|GetKillImpulse (Variables|/Game/BluePrints/Characters/BP_PlayerCharacter.BP_PlayerCharacter_C|GetCurrentWeapon _playerref)))) ImpactPoint BoneName)
  (if (Utilities|IsValid _capsulecomponent)
    (Components|DestroyComponent _capsulecomponent)))