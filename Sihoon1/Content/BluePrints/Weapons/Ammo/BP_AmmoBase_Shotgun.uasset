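; Shotgun ammo projectile Blueprint that takes its speed from shared game data.
; On BeginPlay it runs the parent logic, then sets the ProjectileMovement initial speed from the ShotgunAmmoData held in BP_GameInstance.
; All other behavior comes from the parent class, as its construction script only calls the parent and its overlap and tick events are disabled.
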(event EventBeginPlay
  (|CallParentFunction)
  (bind _asbp_game_instance (Utilities|Casting|CastToBP_GameInstance (Game|GetGameInstance)))
  (Variables|/Script/Engine.ProjectileMovementComponent|SetInitialSpeed (Variables|Default|GetProjectileMovement) (.speed (Variables|/Game/BluePrints/BP_GameInstance.BP_GameInstance_C|GetShotgunAmmoData _asbp_game_instance))))

(event Collision|EventActorBeginOverlap
  (params (OtherActor :type Actor%20Object%20Reference))
  (|CallParentFunction OtherActor) ; This node is disabled and will not be called.\nDrag off pins to build functionality.
)

(event EventTick
  (params (DeltaSeconds :type Float%20%28single-precision%29))
  (|CallParentFunction DeltaSeconds) ; This node is disabled and will not be called.\nDrag off pins to build functionality.
)

(fn ConstructionScript
  (|CallParentFunction))