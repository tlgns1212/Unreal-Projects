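; Sniper rifle weapon Blueprint that extends a parent weapon with rifle-specific ammo data, firing effects and a scope view.
; BeginPlay pulls its ammo data from BP_GameInstance; firing plays the gun animation, then applies automatic recoil when aiming or ejects a shell effect otherwise.
; Aiming blocks switching and reloading, then after a short delay shows the scope widget and hides the gun, pawn and HUD.
; Exiting aim reverses these changes.
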(event EventBeginPlay
  (|CallParentFunction)
  (bind _asbp_game_instance (Utilities|Casting|CastToBP_GameInstance (Game|GetGameInstance)))
  (Variables|Default|SetAmmoData (Variables|/Game/BluePrints/BP_GameInstance.BP_GameInstance_C|GetSniperRifleAmmoData _asbp_game_instance)))

(event EventWeaponFire
  (params (AmmoActor :type Actor%20Class%20Reference) (FireType :type FireType%20Enum :default "NewEnumerator0"))
  (bind _gunmesh (Variables|Default|GetGunMesh))
  (bind _returnvalue (Transformation|GetSocketTransform _gunmesh "AmmoEject" "RTS_World"))
  (|CallParentFunction AmmoActor FireType)
  (Components|Animation|PlayAnimation (Variables|Default|GetGunMesh) "/Game/MilitaryWeapSilver/Weapons/Animations/Fire_SniperRifle_W.Fire_SniperRifle_W" false)
  (if (Variables|Default|GetIsAiming)
    (CallFunction|AutomaticRecoil)
    (else
      (Effects|SpawnEmitteratLocation "/Game/BluePrints/Particles/FX_SniperShell.FX_SniperShell" (.location _returnvalue) (.rotation _returnvalue)))))

(event EventOnAimEnter
  (bind _playerref (Variables|Default|GetPlayerRef))
  (bind _playerref_2 (Variables|Default|GetPlayerRef))
  (bind _sniperscoperef (Variables|/Game/BluePrints/Characters/BP_PlayerCharacter.BP_PlayerCharacter_C|GetSniperScopeRef _playerref))
  ;[1 1 1] AimEnter Event
  (|CallParentFunction)
  (if (== (Variables|/Game/BluePrints/Characters/BP_PlayerCharacter.BP_PlayerCharacter_C|GetCurrentWeapon (Variables|Default|GetPlayerRef)) self)
    (Variables|/Game/BluePrints/Characters/BP_PlayerCharacter.BP_PlayerCharacter_C|SetCanSwitchWeapon _playerref_2 false)
    (Variables|/Game/BluePrints/Characters/BP_PlayerCharacter.BP_PlayerCharacter_C|SetCanReload _playerref_2 false)
    (Utilities|FlowControl|Delay 0.1)
    (if (not (UserInterface|Viewport|IsinViewport _sniperscoperef))
      (UserInterface|Viewport|AddtoViewport _sniperscoperef 0)
      (Development|SetHiddeninGame (Variables|Default|GetGunMesh) true false)
      (Rendering|SetActorHiddenInGame (Game|Player|GetPlayerPawn 0) true)
      (Widget|SetVisibility (Variables|/Game/BluePrints/Characters/BP_PlayerCharacter.BP_PlayerCharacter_C|GetMainHUDRef (Variables|Default|GetPlayerRef)) "Collapsed"))))

(event EventOnAimExit
  (bind _playerref (Variables|Default|GetPlayerRef))
  ;[1 1 1] AimExit Event
  (|CallParentFunction)
  (Variables|/Game/BluePrints/Characters/BP_PlayerCharacter.BP_PlayerCharacter_C|SetCanSwitchWeapon _playerref true)
  (Variables|/Game/BluePrints/Characters/BP_PlayerCharacter.BP_PlayerCharacter_C|SetCanReload _playerref true)
  (Widget|RemovefromParent (Variables|/Game/BluePrints/Characters/BP_PlayerCharacter.BP_PlayerCharacter_C|GetSniperScopeRef _playerref))
  (Development|SetHiddeninGame (Variables|Default|GetGunMesh) false false)
  (Rendering|SetActorHiddenInGame (Game|Player|GetPlayerPawn 0) false)
  (Widget|SetVisibility (Variables|/Game/BluePrints/Characters/BP_PlayerCharacter.BP_PlayerCharacter_C|GetMainHUDRef (Variables|Default|GetPlayerRef)) "Visible"))

(fn ConstructionScript
  (|CallParentFunction))