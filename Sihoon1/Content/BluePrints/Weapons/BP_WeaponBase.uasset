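; Base player weapon that handles hitscan or projectile firing, magazine and reserve ammo, and aim state from player events.
; CalculateShot traces from the camera with random spread and orients a muzzle-socket transform toward the impact for projectiles.
; Hitscan shots spawn impact effects and send damage messages, while projectiles receive the damage data on spawn.
; Automatic weapons play timeline-driven controller recoil that reverses, and Tick drives the player's ADS FOV.
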(event Custom|AutomaticRecoil
  (bind _returnvalue (Game|Player|GetPlayerPawn 0))
  ;[1 1 1] RecoilControllerPicthAndYawForAutomaticWeapons
  (bind (_direction _alpha) (Timeline|RecoilTimeline PlayFromStart)
    (:Update
      (switch Utilities|FlowControl|Switch|SwitchonETimelineDirection _direction
        (:Forward
          (Pawn|Input|AddControllerPitchInput _returnvalue (Math|Float|Lerp 0.0 (Variables|Recoil|GetRecoilPitch) _alpha))
          (Pawn|Input|AddControllerYawInput _returnvalue (Math|Random|RandomFloatinRange -0.15 0.15)))
        (:Backward
          (Pawn|Input|AddControllerPitchInput _returnvalue (* (Math|Float|Lerp 0.0 (Variables|Recoil|GetRecoilPitch) _alpha) -1.0)))))
    (:Finished
      (CallFunction|ReverseRecoil)
      (Utilities|FlowControl|RetriggerableDelay 0.05)
      (CallFunction|StopRecoil))))

(event Custom|StopRecoil
  (bind _returnvalue (Game|Player|GetPlayerPawn 0))
  ;[1 1 1] RecoilControllerPicthAndYawForAutomaticWeapons
  (bind (_direction _alpha) (Timeline|RecoilTimeline Stop)
    (:Update
      (switch Utilities|FlowControl|Switch|SwitchonETimelineDirection _direction
        (:Forward
          (Pawn|Input|AddControllerPitchInput _returnvalue (Math|Float|Lerp 0.0 (Variables|Recoil|GetRecoilPitch) _alpha))
          (Pawn|Input|AddControllerYawInput _returnvalue (Math|Random|RandomFloatinRange -0.15 0.15)))
        (:Backward
          (Pawn|Input|AddControllerPitchInput _returnvalue (* (Math|Float|Lerp 0.0 (Variables|Recoil|GetRecoilPitch) _alpha) -1.0)))))
    (:Finished
      (CallFunction|ReverseRecoil)
      (Utilities|FlowControl|RetriggerableDelay 0.05)
      (CallFunction|StopRecoil))))

(event Custom|ReverseRecoil
  (bind _returnvalue (Game|Player|GetPlayerPawn 0))
  ;[1 1 1] RecoilControllerPicthAndYawForAutomaticWeapons
  (bind (_direction _alpha) (Timeline|RecoilTimeline Reverse)
    (:Update
      (switch Utilities|FlowControl|Switch|SwitchonETimelineDirection _direction
        (:Forward
          (Pawn|Input|AddControllerPitchInput _returnvalue (Math|Float|Lerp 0.0 (Variables|Recoil|GetRecoilPitch) _alpha))
          (Pawn|Input|AddControllerYawInput _returnvalue (Math|Random|RandomFloatinRange -0.15 0.15)))
        (:Backward
          (Pawn|Input|AddControllerPitchInput _returnvalue (* (Math|Float|Lerp 0.0 (Variables|Recoil|GetRecoilPitch) _alpha) -1.0)))))
    (:Finished
      (CallFunction|ReverseRecoil)
      (Utilities|FlowControl|RetriggerableDelay 0.05)
      (CallFunction|StopRecoil))))

(event Custom|OnAimEnter
  (Variables|ADS|SetIsAiming true))

(event Custom|OnAimExit
  (Variables|ADS|SetIsAiming false))

(event EventBeginPlay
  (bind _asbp_player_character (Utilities|Casting|CastToBP_PlayerCharacter (Game|Player|GetPlayerPawn 0)))
  (Variables|References|SetPlayerRef _asbp_player_character)
  (EventDispatchers|AssignAimEnter _asbp_player_character (delegate Custom|OnAimEnter))
  (EventDispatchers|AssignAimExit _asbp_player_character (delegate Custom|OnAimExit)))

(event EventTick
  (params (DeltaSeconds :type Float%20%28single-precision%29))
  (Default|ADSFOV (Variables|References|GetPlayerRef)))

(fn ConstructionScript)

(fn WeaponFire
  (params (AmmoActor :type Actor%20Class%20Reference) (FireType :type FireType%20Enum :default "NewEnumerator0"))
  (bind _playerref (Variables|References|GetPlayerRef))
  (bind _playerref_2 (Variables|References|GetPlayerRef))
  (Variables|Ammo|SetCurrentAmmo (- (Variables|Ammo|GetCurrentAmmo) 1))
  (switch Utilities|FlowControl|Switch|SwitchonFireType FireType
    (:NewEnumerator0
      (if (Variables|Ammo|GetIsMultipleBullets)
        (for _index (range 0 (- (Variables|Ammo|GetBulletCount) 1))
          (bind _hitresult (CallFunction|CalculateShot (Variables|/Game/BluePrints/Characters/BP_PlayerCharacter.BP_PlayerCharacter_C|GetUnusedCamera _playerref) (Variables|Components|GetGunMesh) "MuzzleFlash" (Variables|/Game/BluePrints/Characters/BP_PlayerCharacter.BP_PlayerCharacter_C|GetCamera _playerref) AmmoActor))
          (Game|SpawnActorfromClass (Variables|Properties|GetImpactEffectClass) (Math|Transform|MakeTransform (.ImpactNormal (Collision|BreakHitResult _hitresult)) "0, 0, 0" "1.000000,1.000000,1.000000") "Undefined" 0 _hitresult (.bBlockingHit (Collision|BreakHitResult _hitresult)) 0)
          (CallFunction|AddDamage _hitresult)
          (if (Variables|Properties|GetIsAutomaticWeapon)
            (CallFunction|AutomaticRecoil)))
        (else
          (bind _hitresult_2 (CallFunction|CalculateShot (Variables|/Game/BluePrints/Characters/BP_PlayerCharacter.BP_PlayerCharacter_C|GetUnusedCamera _playerref) (Variables|Components|GetGunMesh) "MuzzleFlash" (Variables|/Game/BluePrints/Characters/BP_PlayerCharacter.BP_PlayerCharacter_C|GetCamera _playerref) AmmoActor))
          (Game|SpawnActorfromClass (Variables|Properties|GetImpactEffectClass) (Math|Transform|MakeTransform (.ImpactNormal (Collision|BreakHitResult _hitresult_2)) "0, 0, 0" "1.000000,1.000000,1.000000") "Undefined" 0 _hitresult_2 (.bBlockingHit (Collision|BreakHitResult _hitresult_2)) 0)
          (CallFunction|AddDamage _hitresult_2)
          (if (Variables|Properties|GetIsAutomaticWeapon) :!label _label
            (CallFunction|AutomaticRecoil)))))
    (:NewEnumerator1
      (bind _projectiletransform (CallFunction|CalculateShot (Variables|/Game/BluePrints/Characters/BP_PlayerCharacter.BP_PlayerCharacter_C|GetUnusedCamera _playerref_2) (Variables|Components|GetGunMesh) "MuzzleFlash" (Variables|/Game/BluePrints/Characters/BP_PlayerCharacter.BP_PlayerCharacter_C|GetCamera _playerref_2) AmmoActor))
      (bind _returnvalue (Game|SpawnActorfromClass (Variables|Projectile|GetProjectile) _projectiletransform "AlwaysSpawn" 0 (Variables|Properties|GetAmmoData) (Variables|Stats|GetCriticalHitDamageModifier) 0))
      (Variables|Projectile|SetSpawnedProjectile _returnvalue)
      (goto _label))))

(fn WeaponReload
  (Variables|Ammo|SetCurrentAmmo (Math|Integer|Min(Integer) (Variables|Ammo|GetMaxMagAmmo) (Variables|Ammo|GetCurrentTotalAmmo)))
  (Variables|Ammo|SetCurrentTotalAmmo (- (Variables|Ammo|GetCurrentTotalAmmo) (Math|Integer|Min(Integer) (Variables|Ammo|GetMaxMagAmmo) (Variables|Ammo|GetCurrentTotalAmmo)))))

(fn HasAmmoinMag
  (return (> (Variables|Ammo|GetCurrentAmmo) 0) (== (Variables|Ammo|GetCurrentAmmo) (Variables|Ammo|GetMaxMagAmmo))))

(fn HasExtraAmmo
  (return (> (Variables|Ammo|GetCurrentTotalAmmo) 0)))

(fn CalculateShot
  (params (UnusedCamera :type Camera%20Component%20Object%20Reference) (WeaponMesh :type Scene%20Component%20Object%20Reference) (WeaponFireSocketName :type Name) (Camera :type Camera%20Component%20Object%20Reference) (AmmoActor :type Actor%20Class%20Reference))
  (bind _bulletspread (Variables|Stats|GetBulletSpread))
  (bind _returnvalue (* _bulletspread -1.0))
  (Utilities|FlowControl|Sequence
    (:then_0
      (LocalVariables|SetLocalUnusedCamera UnusedCamera)
      (LocalVariables|SetLocalWeaponMesh WeaponMesh)
      (LocalVariables|SetLocalSocketName WeaponFireSocketName)
      (LocalVariables|SetLocalCamera Camera))
    (:then_1
      (bind (_outhit _returnvalue_2) (Collision|LineTraceForObjects (.location (Transformation|GetWorldTransform (LocalVariables|GetLocalCamera))) (Math|Vector|MakeVector (+ (.X (Math|Vector|BreakVector (+ (.location (Transformation|GetWorldTransform (LocalVariables|GetLocalCamera))) (* (Math|Vector|GetForwardVector (Math|Rotator|MakeRotator (.roll (.rotation (Transformation|GetWorldTransform (LocalVariables|GetLocalCamera)))) (+ (.pitch (.rotation (Transformation|GetWorldTransform (LocalVariables|GetLocalCamera)))) 5.0) (.yaw (.rotation (Transformation|GetWorldTransform (LocalVariables|GetLocalCamera)))))) (Variables|Stats|GetBulletRange))))) (Math|Random|RandomFloatinRange _returnvalue _bulletspread)) (+ (.Y (Math|Vector|BreakVector (+ (.location (Transformation|GetWorldTransform (LocalVariables|GetLocalCamera))) (* (Math|Vector|GetForwardVector (Math|Rotator|MakeRotator (.roll (.rotation (Transformation|GetWorldTransform (LocalVariables|GetLocalCamera)))) (+ (.pitch (.rotation (Transformation|GetWorldTransform (LocalVariables|GetLocalCamera)))) 5.0) (.yaw (.rotation (Transformation|GetWorldTransform (LocalVariables|GetLocalCamera)))))) (Variables|Stats|GetBulletRange))))) (Math|Random|RandomFloatinRange _returnvalue _bulletspread)) (+ (.Z (Math|Vector|BreakVector (+ (.location (Transformation|GetWorldTransform (LocalVariables|GetLocalCamera))) (* (Math|Vector|GetForwardVector (Math|Rotator|MakeRotator (.roll (.rotation (Transformation|GetWorldTransform (LocalVariables|GetLocalCamera)))) (+ (.pitch (.rotation (Transformation|GetWorldTransform (LocalVariables|GetLocalCamera)))) 5.0) (.yaw (.rotation (Transformation|GetWorldTransform (LocalVariables|GetLocalCamera)))))) (Variables|Stats|GetBulletRange))))) (Math|Random|RandomFloatinRange _returnvalue _bulletspread))) (Utilities|Array|MakeArray "ObjectTypeQuery1" "ObjectTypeQuery2") false (Utilities|Array|MakeArray (Game|Player|GetPlayerPawn 0)) "None"))
      (if _returnvalue_2
        (LocalVariables|SetLocalProjectileTransform (Math|Transform|MakeTransform (Transformation|GetSocketLocation (LocalVariables|GetLocalWeaponMesh) (LocalVariables|GetLocalSocketName)) (Math|Rotator|FindLookatRotation (Transformation|GetSocketLocation (LocalVariables|GetLocalWeaponMesh) (LocalVariables|GetLocalSocketName)) (.ImpactPoint (Collision|BreakHitResult _outhit)))))
        (else
          (LocalVariables|SetLocalProjectileTransform (Math|Transform|MakeTransform (Transformation|GetSocketLocation (LocalVariables|GetLocalWeaponMesh) (LocalVariables|GetLocalSocketName)) (Pawn|GetControlRotation (.AsPawn (Utilities|Casting|CastToPawn (Components|GetOwner (LocalVariables|GetLocalCamera)))) :!class /Script/Engine.Pawn))))))
    (:then_2
      (return _outhit (LocalVariables|GetLocalProjectileTransform)))))

(fn AddDamage
  (params (HitResult :type Hit%20Result%20Structure))
  (Class|TakeDamage|TakeDamage(Message) (.HitActor (Collision|BreakHitResult HitResult)) (Variables|Properties|GetAmmoData) (Variables|Stats|GetCriticalHitDamageModifier) HitResult))

(fn StopFire)