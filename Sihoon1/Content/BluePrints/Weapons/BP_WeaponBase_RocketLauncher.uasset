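; Rocket launcher weapon Blueprint that extends a parent weapon class with launcher-specific ammo data and fire feedback.
; On BeginPlay it pulls its rocket launcher ammo data from BP_GameInstance.
; On WeaponFire it runs the parent firing logic, then plays the gun mesh fire animation and a world camera shake centered on the weapon's location.
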(event EventBeginPlay
  (|CallParentFunction)
  (bind _asbp_game_instance (Utilities|Casting|CastToBP_GameInstance (Game|GetGameInstance)))
  (Variables|Default|SetAmmoData (Variables|/Game/BluePrints/BP_GameInstance.BP_GameInstance_C|GetRocketLauncherAmmoData _asbp_game_instance)))

(event EventWeaponFire
  (params (AmmoActor :type Actor%20Class%20Reference) (FireType :type FireType%20Enum :default "NewEnumerator0"))
  (|CallParentFunction AmmoActor FireType)
  (Components|Animation|PlayAnimation (Variables|Default|GetGunMesh) "/Game/MilitaryWeapSilver/Weapons/Animations/Fire_RocketLauncher_W.Fire_RocketLauncher_W" false)
  (Camera|PlayWorldCameraShake "/Game/BluePrints/CameraShakes/RocketLauncherCameraShake.RocketLauncherCameraShake_C" (Transformation|GetActorLocation) 0.0 5e+02))

(fn ConstructionScript
  (|CallParentFunction))