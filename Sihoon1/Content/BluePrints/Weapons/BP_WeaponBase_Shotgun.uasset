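; Shotgun weapon Blueprint that extends its parent weapon's startup and firing with shotgun-specific ammo data, animation and effects.
; On BeginPlay it pulls the shotgun ammo data from BP_GameInstance, then derives reload time in proportion to maximum magazine size.
; Firing runs the parent fire logic with a fixed fire type, then plays the gun mesh fire animation and spawns a shell particle at the AmmoEject socket.
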(event Custom|SetReloadTime
  (Variables|Default|SetReloadTime (* (Variables|Default|GetMaxMagAmmo) 0.5)))

(event EventBeginPlay
  (|CallParentFunction)
  (bind _asbp_game_instance (Utilities|Casting|CastToBP_GameInstance (Game|GetGameInstance)))
  (Variables|Default|SetAmmoData (Variables|/Game/BluePrints/BP_GameInstance.BP_GameInstance_C|GetShotgunAmmoData _asbp_game_instance))
  (CallFunction|SetReloadTime))

(event EventWeaponFire
  (params (AmmoActor :type Actor%20Class%20Reference) (FireType :type FireType%20Enum :default "NewEnumerator0"))
  (bind _gunmesh (Variables|Default|GetGunMesh))
  (bind _returnvalue (Transformation|GetSocketTransform _gunmesh "AmmoEject" "RTS_World"))
  (|CallParentFunction 0 "NewEnumerator0")
  (Components|Animation|PlayAnimation (Variables|Default|GetGunMesh) "/Game/MilitaryWeapSilver/Weapons/Animations/Fire_Shotgun_W.Fire_Shotgun_W" false)
  (Effects|SpawnEmitteratLocation "/Game/BluePrints/Particles/FX_ShotgunShell.FX_ShotgunShell" (.location _returnvalue) (.rotation _returnvalue)))

(fn ConstructionScript
  (|CallParentFunction))