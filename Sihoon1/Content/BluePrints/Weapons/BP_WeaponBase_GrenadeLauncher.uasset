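; Grenade launcher weapon Blueprint that extends a parent weapon class with launcher-specific ammo data and fire animation.
; On BeginPlay it calls the parent, then pulls the grenade launcher ammo data from BP_GameInstance.
; Firing runs the parent fire logic, then plays the launcher's fire animation on the gun mesh.
; A rocket launcher camera shake node is present but never runs.
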(event EventBeginPlay
  (|CallParentFunction)
  (bind _asbp_game_instance (Utilities|Casting|CastToBP_GameInstance (Game|GetGameInstance)))
  (Variables|Default|SetAmmoData (Variables|/Game/BluePrints/BP_GameInstance.BP_GameInstance_C|GetGrenadeLauncherAmmoData _asbp_game_instance)))

(event EventWeaponFire
  (params (AmmoActor :type Actor%20Class%20Reference) (FireType :type FireType%20Enum :default "NewEnumerator0"))
  (|CallParentFunction AmmoActor FireType)
  (Components|Animation|PlayAnimation (Variables|Default|GetGunMesh) "/Game/MilitaryWeapSilver/Weapons/Animations/Fire_GrenadeLauncher_W.Fire_GrenadeLauncher_W" false))

(fn ConstructionScript
  (|CallParentFunction))