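; Assault rifle weapon Blueprint that extends a parent weapon with automatic fire.
; On BeginPlay it pulls rifle ammo data from BP_GameInstance.
; WeaponFire fires immediately, then repeats RifleFire on a looping timer until StopFire clears it.
; Each shot calls the parent fire logic, plays gun and character fire actions, then either ejects a shell effect or, when ammo is empty, stops and reloads.
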(event Custom|RifleFire
  (bind _gunmesh (Variables|Default|GetGunMesh))
  (bind _returnvalue (Transformation|GetSocketTransform _gunmesh "AmmoEject" "RTS_World"))
  ;[1 1 1] RifleFireAndStop
  (if (Variables|Default|GetIsRifleFiring)
    (|CallParentFunction (stale EventWeaponFire AmmoActor) (stale EventWeaponFire FireType))
    (Components|Animation|PlayAnimation (Variables|Default|GetGunMesh) "/Game/MilitaryWeapSilver/Weapons/Animations/Fire_Rifle_W2.Fire_Rifle_W2" false)
    (Default|CallCharacterFireWeapon (Variables|Default|GetPlayerRef) "NewEnumerator1")
    (if (<= (Variables|Default|GetCurrentAmmo) 0)
      (CallFunction|StopFire)
      (Default|Reload (Variables|Default|GetPlayerRef))
      (else
        (Effects|SpawnEmitteratLocation "/Game/BluePrints/Particles/FX_AssaultRifleShell.FX_AssaultRifleShell" (.location _returnvalue) (.rotation _returnvalue))))))

(event EventBeginPlay
  (|CallParentFunction)
  (bind _asbp_game_instance (Utilities|Casting|CastToBP_GameInstance (Game|GetGameInstance)))
  (Variables|Default|SetAmmoData (Variables|/Game/BluePrints/BP_GameInstance.BP_GameInstance_C|GetAssaultRifleAmmoData _asbp_game_instance)))

(event Collision|EventActorBeginOverlap
  (params (OtherActor :type Actor%20Object%20Reference))
  (|CallParentFunction OtherActor) ; This node is disabled and will not be called.\nDrag off pins to build functionality.
)

(event EventTick
  (params (DeltaSeconds :type Float%20%28single-precision%29))
  (|CallParentFunction DeltaSeconds) ; This node is disabled and will not be called.\nDrag off pins to build functionality.
)

(event EventWeaponFire
  (params (AmmoActor :type Actor%20Class%20Reference) (FireType :type FireType%20Enum :default "NewEnumerator0"))
  ;[1 1 1] RifleFireAndStop
  (Variables|Default|SetIsRifleFiring true)
  (CallFunction|RifleFire)
  (bind _returnvalue (Utilities|Time|SetTimerbyEvent (delegate Custom|RifleFire) (Variables|Default|GetAutomaticFireRate) true))
  (Variables|Default|SetRifleFireTimerHandle _returnvalue))

(event EventStopFire
  ;[1 1 1] RifleFireAndStop
  (|CallParentFunction)
  (Variables|Default|SetIsRifleFiring false)
  (Utilities|Time|ClearandInvalidateTimerbyHandle (Variables|Default|GetRifleFireTimerHandle)))

(fn ConstructionScript
  (|CallParentFunction))