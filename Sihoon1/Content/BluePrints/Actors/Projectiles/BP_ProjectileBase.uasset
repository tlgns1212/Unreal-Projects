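; Base Blueprint for projectiles, handling what happens when the ProjectileMovement component stops on an impact.
; Unless flagged as causing radius damage, it sends the hit actor a TakeDamageMessage with ammo data, critical modifier and hit result.
; It always hides the mesh, spawns the ImpactEffect actor at the mesh transform with the hit result, then expires via a short lifespan.
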(event OnProjectileStop(ProjectileMovement)
  (params (ImpactResult :type Hit%20Result%20Structure%20%28by%20ref%29))
  (CallFunction|ProjectileStop ImpactResult))

(fn ConstructionScript)

(fn ProjectileStop
  (params (HitResult :type Hit%20Result%20Structure))
  (bind _mesh (Variables|Default|GetMesh))
  (Utilities|FlowControl|Sequence
    (:then_0
      (if (not (Variables|Default|GetiscausingRadiusDamage))
        (Class|TakeDamage|TakeDamage(Message) (.HitActor (Collision|BreakHitResult HitResult)) (Variables|Default|GetAmmoData) (Variables|Default|GetCriticalDamageModifier) HitResult)))
    (:then_1
      (Development|SetHiddeninGame _mesh true false)
      (Game|SpawnActorfromClass (Variables|Default|GetImpactEffect) (Transformation|GetWorldTransform _mesh) "AlwaysSpawn" 0 HitResult true 0)
      (Actor|SetLifeSpan 0.1))))